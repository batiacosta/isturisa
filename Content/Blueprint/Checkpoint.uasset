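; Checkpoint actor whose static mesh attaches visually to an actor inside its box trigger, then returns home.
; BeginPlay saves the mesh's transform, and box overlap starts audio and enables following.
; While enabled, Tick moves the mesh to the overlapping actor's first static mesh component tagged PlaceForSigns and shrinks it.
; Ending overlap restores the saved transform and stops following, with no filter on actor type.
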(event OnComponentBeginOverlap(Box)
  (params (OverlappedComponent :type Primitive%20Component%20Object%20Reference) (OtherActor :type Actor%20Object%20Reference) (OtherComp :type Primitive%20Component%20Object%20Reference) (OtherBodyIndex :type Integer) (bFromSweep :type Boolean) (SweepResult :type Hit%20Result%20Structure%20%28by%20ref%29))
  (Variables|Default|SetCanMove true)
  (Audio|Components|Audio|Play (Variables|Default|GetAudio) 0.0))

(event OnComponentEndOverlap(Box)
  (params (OverlappedComponent :type Primitive%20Component%20Object%20Reference) (OtherActor :type Actor%20Object%20Reference) (OtherComp :type Primitive%20Component%20Object%20Reference) (OtherBodyIndex :type Integer))
  (Transformation|SetWorldTransform (Variables|Default|GetStaticMesh) (Variables|Default|GetStartLocation) false false)
  (Variables|Default|SetCanMove false))

(event EventBeginPlay
  (Variables|Default|SetStartLocation (Transformation|GetWorldTransform (Variables|Default|GetStaticMesh))))

(event Collision|EventActorBeginOverlap
  (params (OtherActor :type Actor%20Object%20Reference)))

(event EventTick
  (params (DeltaSeconds :type Float%20%28single-precision%29))
  (bind _staticmesh (Variables|Default|GetStaticMesh))
  (if (Variables|Default|GetCanMove)
    (Transformation|SetWorldLocation _staticmesh (Transformation|GetWorldLocation (Utilities|Array|Get(acopy) (Actor|GetComponentsbyTag (stale OnComponentBeginOverlap(Box) OtherActor) "/Script/Engine.StaticMeshComponent" "PlaceForSigns"))) false false)
    (Transformation|SetWorldScale3D _staticmesh "0.400000,0.400000,0.400000")))

(fn ConstructionScript)